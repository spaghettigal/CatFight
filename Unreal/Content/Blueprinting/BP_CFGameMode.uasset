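; BP_CFGameMode is a game mode that runs an on-screen countdown when play begins.
; BeginPlay creates the Countdown widget, adds it to the viewport and starts a looping one-second timer.
; Each tick of the timer decrements Count and updates the widget text; at zero it clears the timer, removes the widget and plays a boxing bell sound.
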(event `self.ReceiveBeginPlay`
  (bind _returnvalue (`|CreateWidget` "/Game/UI/countdown.countdown_C"))
  (bind _output_get (set `self.countdown widget` _returnvalue))
  (`UserWidget.AddToViewport` _output_get 0)
  (bind _returnvalue_2 (`KismetSystemLibrary.K2_SetTimerDelegate` (delegate `take countdown`) 1.0 true)))

(event `take countdown`
  (`/Engine/EditorBlueprintResources/StandardMacros.DecrementInt` (`self.count`)
    (:`  `
      (`TextBlock.SetText` (`/Game/UI/countdown.countdowntext` (`self.countdown widget`)) (`KismetTextLibrary.Conv_IntToText` (`self.count`)))
      (if (<= (`self.count`) 0)
        (`KismetSystemLibrary.K2_ClearAndInvalidateTimerHandle` (stale `self.ReceiveBeginPlay` _returnvalue_2))
        (`Widget.RemoveFromParent` (`self.countdown widget`))
        (`GameplayStatics.PlaySound2D` "/Game/ART/Music+Sounds/mateusz-chenc-boxing-bell-signals_01ymQnyW_Cue.mateusz-chenc-boxing-bell-signals_01ymQnyW_Cue" 1.0 1.0 0.0 null null)))))

(fn `UserConstructionScript`)