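; BP_CFAIEnemy is a melee enemy character that chases the player and takes damage until it dies.
; BeginPlay caches the player, plays one random punch montage, then starts a self-repeating AIMoveTo chase.
; onHit uses DoOnce to block repeat hits during the impact montage, then subtracts Damage from Health, resetting or playing a random death montage before destruction.
; AIKicking and AICrouch are empty stubs, and both hand-based impact choices use the same montage.
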(event `self.ReceiveBeginPlay`
  (bind _asbp_cfplayer_1 (cast `/Game/Blueprinting/BP_CFPlayer1` (`GameplayStatics.GetPlayerCharacter` 0)))
  (set `self.CharacterRef` _asbp_cfplayer_1)
  (`self.AIPunching`)
  (`KismetSystemLibrary.Delay` 2.0)
  (`self.ChasePlayer`))

(event `ChasePlayer`
  (`|AIMoveTo` self (0.0 0.0 0.0) (`GameplayStatics.GetPlayerCharacter` 0) 100.0
    (:`then`
      _)
    (:`OnSuccess`
      _))
  (`KismetSystemLibrary.Delay` 1.0)
  (`self.ChasePlayer`))

(event `onHit`
  (`/Engine/EditorBlueprintResources/StandardMacros.DoOnce` false :!label _label
    (:`Completed`
      (`GameplayStatics.PlaySoundAtLocation` null (`self.K2_GetActorLocation`) (struct) 1.0 1.0 0.0 null null null null) ; Add cat sounds to this when we have aduio
      (bind _returnvalue (`self.PlayAnimMontage` (select `bool` (`/Game/Blueprinting/BP_CFPlayer1.Right Hand?` (`self.CharacterRef`)) :`false` "/Game/Characters/Mannequins/Animations/CatFightPlayer1/Impact_mixamo_com_Montage.Impact_mixamo_com_Montage" :`true` "/Game/Characters/Mannequins/Animations/CatFightPlayer1/Impact_mixamo_com_Montage.Impact_mixamo_com_Montage" :!type "AnimMontage Object Reference")))
      (`KismetSystemLibrary.Delay` _returnvalue)
      (bind _output_get (set `self.Health` (- (`self.Health`) (`self.Damage`))))
      (if (<= _output_get 0)
        (`GameplayStatics.PlaySoundAtLocation` null (`self.K2_GetActorLocation`) (struct) 1.0 1.0 0.0 null null null null) ; DeathSoundAffect
        (bind _returnvalue_2 (`self.PlayAnimMontage` (`|GetArrayItem` (`self.Anim Montage`) (`KismetMathLibrary.RandomIntegerInRange` 0 2))))
        (`KismetSystemLibrary.Delay` _returnvalue_2)
        (`self.K2_DestroyActor`)
        (else
          (goto _label :!via `Reset`))))))

(event `AIKicking`)

(event `AICrouch`)

(event `AIPunching`
  (`self.PlayAnimMontage` (`|GetArrayItem` (`self.Montage to Play`) (`KismetMathLibrary.RandomIntegerInRange` 0 2))))

(fn `UserConstructionScript`)